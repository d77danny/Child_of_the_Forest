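; BP_Witch is the player character, with third-person movement, jumping, an interact call and box pushing.
; Overlapping a Pushing_Box opens four side gates; E then runs a timeline snapping the player to that side's point and arrow rotation.
; Looping timers interpolate the box ahead of the player until R releases it.
; While pushing, jumping is blocked and W sets forward push scale; a sphere-trace collision check is left unconnected.
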(event `self.ReceiveTick`
  (params (DeltaSeconds :type "Float (single-precision)"))
  ;[1 1 1] Box PickUp
)

(event `Key|W`
  (params (Key :type "Key Structure"))
  ;[1 1 1] Box PickUp
  ;;[1 1 1] Box PickUp Button Bindings
  (:`Pressed`
    (set `self.SetForwardPushVelocity` 1.0))
  (:`Released`
    (set `self.SetForwardPushVelocity` 0.0)))

(event `InputAxis|MoveForward`
  (params (AxisValue :type "Float (single-precision)"))
  ;[1 1 1] Box PickUp
  ;;[1 1 1] Box PickUp Movement
  (if (`self.IsPushingObject`)
    (`self.AddMovementInput` (`self.SetPushDirection`) (`self.SetForwardPushVelocity`))
    (else
      (`self.AddMovementInput` (`KismetMathLibrary.GetForwardVector` (`KismetMathLibrary.MakeRotator` 0.0 0.0 (.yaw (`self.GetControlRotation`)))) AxisValue))))

(event `Key|E`
  (params (Key :type "Key Structure"))
  ;[1 1 1] Box PickUp
  ;;[1 1 1] Box PickUp Button Bindings
  (:`Pressed`
    (set `self.EKeyIsPressed` true))
  (:`Released`
    (set `self.EKeyIsPressed` false)))

(event `Key|R`
  (params (Key :type "Key Structure"))
  ;[1 1 1] Box PickUp
  ;;[1 1 1] Box PickUp Button Bindings
  (:`Pressed`
    (set `self.RKeyIsPressed` true))
  (:`Released`
    (set `self.RKeyIsPressed` false)))

(event `InputAxis|MoveRight`
  (params (AxisValue :type "Float (single-precision)"))
  ;[1 1 1] Box PickUp
  ;;[1 1 1] Box PickUp Movement
  (if (not (`self.IsPushingObject`))
    (`self.AddMovementInput` (`KismetMathLibrary.GetForwardVector` (`KismetMathLibrary.MakeRotator` 0.0 0.0 (.yaw (`self.GetControlRotation`)))) AxisValue)))

(event `UpdateLocationPushingBox`
  (bind _returnvalue (`GameplayStatics.GetPlayerCharacter` 0))
  ;[1 1 1] Box PickUp
  ;;[1 1 1] Side 1
  (if true
    (`self.K2_SetActorLocationAndRotation` :`self` (stale `self.ReceiveActorBeginOverlap` _aspushing_box) :`NewLocation` (`KismetMathLibrary.VInterpTo` (`self.K2_GetActorLocation` (stale `self.ReceiveActorBeginOverlap` _aspushing_box)) (- (+ (* (`self.GetActorForwardVector` _returnvalue) 150.0) (`self.K2_GetActorLocation` _returnvalue)) (0.0 0.0 50.0)) (`GameplayStatics.GetWorldDeltaSeconds`)))
    (if (`self.RKeyIsPressed`)
      (`KismetSystemLibrary.K2_ClearAndInvalidateTimerHandle` (stale `Key|E` _returnvalue_5))
      (set `self.IsPushingObject` false))))

(event `Key|E`
  (params (Key :type "Key Structure"))
  (bind _returnvalue (`GameplayStatics.GetPlayerCharacter` 0))
  (bind _returnvalue_2 (`GameplayStatics.GetPlayerCharacter` 0))
  (bind _returnvalue_3 (`GameplayStatics.GetPlayerCharacter` 0))
  (bind _returnvalue_4 (`GameplayStatics.GetPlayerCharacter` 0))
  ;[1 1 1] Box PickUp
  (:`Pressed`
    (`|ExecutionSequence`
      (:`then_0`
        ;;[1 1 1] Side 1
        (`/Engine/EditorBlueprintResources/StandardMacros.Gate` true :!label _label
          (:`Exit`
            (if (`/Game/Blueprints/Pushing_Box.Side_1` (stale `self.ReceiveActorBeginOverlap` _aspushing_box))
              (set `self.IsPushingObject` true)
              (bind (_direction _alpha) (`Timeline|Transition` :!via `PlayFromStart`)
                (:`Update`
                  (`self.K2_SetActorLocationAndRotation` _returnvalue_2 (`KismetMathLibrary.VLerp` (`self.K2_GetActorLocation` _returnvalue_2) (`SceneComponent.K2_GetComponentLocation` (`/Game/Blueprints/Pushing_Box.TPPoint1` (stale `self.ReceiveActorBeginOverlap` _aspushing_box))) _alpha) (`KismetMathLibrary.RLerp` (`self.K2_GetActorRotation` _returnvalue_2) (`SceneComponent.K2_GetComponentRotation` (`/Game/Blueprints/Pushing_Box.Arrow_1` (stale `self.ReceiveActorBeginOverlap` _aspushing_box))) _alpha) false false)
                  (bind _returnvalue_5 (`KismetSystemLibrary.K2_SetTimerDelegate` (delegate `UpdateLocationPushingBox`) 0.005 true))))))))
      (:`then_1`
        ;;[1 1 1] Side 2
        (`/Engine/EditorBlueprintResources/StandardMacros.Gate` true :!label _label_2
          (:`Exit`
            (if (`/Game/Blueprints/Pushing_Box.Side_2` (stale `self.ReceiveActorBeginOverlap` _aspushing_box_2))
              (set `self.IsPushingObject` true)
              (bind (_direction_2 _alpha_2) (`Timeline|Timeline_0` :!via `PlayFromStart`)
                (:`Update`
                  (`self.K2_SetActorLocationAndRotation` _returnvalue_3 (`KismetMathLibrary.VLerp` (`self.K2_GetActorLocation` _returnvalue_3) (`SceneComponent.K2_GetComponentLocation` (`/Game/Blueprints/Pushing_Box.TPPoint2` (stale `self.ReceiveActorBeginOverlap` _aspushing_box_2))) _alpha_2) (`KismetMathLibrary.RLerp` (`self.K2_GetActorRotation` _returnvalue_3) (`SceneComponent.K2_GetComponentRotation` (`/Game/Blueprints/Pushing_Box.Arrow_2` (stale `self.ReceiveActorBeginOverlap` _aspushing_box_2))) _alpha_2) false false)
                  (bind _returnvalue_6 (`KismetSystemLibrary.K2_SetTimerDelegate` (delegate `UpdateLocationPushingBox2`) 0.005 true))))))))
      (:`then_2`
        ;;[1 1 1] Side 3
        (`/Engine/EditorBlueprintResources/StandardMacros.Gate` true :!label _label_3
          (:`Exit`
            (if (`/Game/Blueprints/Pushing_Box.Side_3` (stale `self.ReceiveActorBeginOverlap` _aspushing_box_3))
              (set `self.IsPushingObject` true)
              (bind (_direction_3 _alpha_3) (`Timeline|Timeline_1` :!via `PlayFromStart`)
                (:`Update`
                  (`self.K2_SetActorLocationAndRotation` _returnvalue_4 (`KismetMathLibrary.VLerp` (`self.K2_GetActorLocation` _returnvalue_4) (`SceneComponent.K2_GetComponentLocation` (`/Game/Blueprints/Pushing_Box.TPPoint_3` (stale `self.ReceiveActorBeginOverlap` _aspushing_box_3))) _alpha_3) (`KismetMathLibrary.RLerp` (`self.K2_GetActorRotation` _returnvalue_4) (`SceneComponent.K2_GetComponentRotation` (`/Game/Blueprints/Pushing_Box.Arrow_3` (stale `self.ReceiveActorBeginOverlap` _aspushing_box_3))) _alpha_3) false false)
                  (bind _returnvalue_7 (`KismetSystemLibrary.K2_SetTimerDelegate` (delegate `UpdateLocationPushingBox3`) 0.005 true))))))))
      (:`then_3`
        ;;[1 1 1] Side 4
        (`/Engine/EditorBlueprintResources/StandardMacros.Gate` true :!label _label_4
          (:`Exit`
            (if (`/Game/Blueprints/Pushing_Box.Side_4` (stale `self.ReceiveActorBeginOverlap` _aspushing_box_4))
              (set `self.IsPushingObject` true)
              (bind (_direction_4 _alpha_4) (`Timeline|Timeline_2` :!via `PlayFromStart`)
                (:`Update`
                  (`self.K2_SetActorLocationAndRotation` _returnvalue (`KismetMathLibrary.VLerp` (`self.K2_GetActorLocation` _returnvalue) (`SceneComponent.K2_GetComponentLocation` (`/Game/Blueprints/Pushing_Box.TPPoint 4` (stale `self.ReceiveActorBeginOverlap` _aspushing_box_4))) _alpha_4) (`KismetMathLibrary.RLerp` (`self.K2_GetActorRotation` _returnvalue) (`SceneComponent.K2_GetComponentRotation` (`/Game/Blueprints/Pushing_Box.Arrow_4` (stale `self.ReceiveActorBeginOverlap` _aspushing_box_4))) _alpha_4) false false)
                  (bind _returnvalue_8 (`KismetSystemLibrary.K2_SetTimerDelegate` (delegate `UpdateLocationPushingBox4`) 0.005 true)))))))))))

(event `InputAction|Jump`
  (params (Key :type "Key Structure"))
  ;[1 1 1] Jumping
  (:`Pressed`
    (if (not (`self.IsPushingObject`))
      (`self.Jump`)))
  (:`Released`
    (`self.StopJumping`)))

(event `InputAxis|MoveForward`
  (params (AxisValue :type "Float (single-precision)"))
  ;[1 1 1] 3rd Person Movement
  (`self.AddMovementInput` (`KismetMathLibrary.GetForwardVector` (`KismetMathLibrary.MakeRotator` 0.0 0.0 (.yaw (`self.GetControlRotation`)))) AxisValue))

(event `UpdateLocationPushingBox2`
  (bind _returnvalue (`GameplayStatics.GetPlayerCharacter` 0))
  ;[1 1 1] Box PickUp
  ;;[1 1 1] Side 2
  (if true
    (`self.K2_SetActorLocationAndRotation` :`self` (stale `self.ReceiveActorBeginOverlap` _aspushing_box_2) :`NewLocation` (`KismetMathLibrary.VInterpTo` (`self.K2_GetActorLocation` (stale `self.ReceiveActorBeginOverlap` _aspushing_box_2)) (- (+ (* (`self.GetActorForwardVector` _returnvalue) 150.0) (`self.K2_GetActorLocation` _returnvalue)) (0.0 0.0 50.0)) (`GameplayStatics.GetWorldDeltaSeconds`)))
    (if (`self.RKeyIsPressed`)
      (`KismetSystemLibrary.K2_ClearAndInvalidateTimerHandle` (stale `Key|E` _returnvalue_6))
      (set `self.IsPushingObject` false))))

(event `InputAxis|MoveRight`
  (params (AxisValue :type "Float (single-precision)"))
  ;[1 1 1] 3rd Person Movement
  (`self.AddMovementInput` (`KismetMathLibrary.GetRightVector` (`KismetMathLibrary.MakeRotator` 0.0 0.0 (.yaw (`self.GetControlRotation`)))) AxisValue))

(event `self.ReceiveActorBeginOverlap`
  (params (OtherActor :type "Actor Object Reference"))
  ;[1 1 1] Box PickUp
  (`|ExecutionSequence`
    (:`then_0`
      (bind _aspushing_box (cast `/Game/Blueprints/Pushing_Box` OtherActor))
      (goto _label :!via `Open`))
    (:`then_1`
      (bind _aspushing_box_2 (cast `/Game/Blueprints/Pushing_Box` OtherActor))
      (goto _label_2 :!via `Open`))
    (:`then_2`
      (bind _aspushing_box_3 (cast `/Game/Blueprints/Pushing_Box` OtherActor))
      (goto _label_3 :!via `Open`))
    (:`then_3`
      (bind _aspushing_box_4 (cast `/Game/Blueprints/Pushing_Box` OtherActor))
      (goto _label_4 :!via `Open`))))

(event `InputAxis|Turn`
  (params (AxisValue :type "Float (single-precision)"))
  ;[1 1 1] 3rd Person Movement
  (`self.AddControllerYawInput` AxisValue))

(event `InputAction|Interact`
  (params (Key :type "Key Structure"))
  (:`Pressed`
    (`self.Interact`)))

(event `UpdateLocationPushingBox3`
  (bind _returnvalue (`GameplayStatics.GetPlayerCharacter` 0))
  ;[1 1 1] Box PickUp
  ;;[1 1 1] Side 3
  (if true
    (`self.K2_SetActorLocationAndRotation` :`self` (stale `self.ReceiveActorBeginOverlap` _aspushing_box_3) :`NewLocation` (`KismetMathLibrary.VInterpTo` (`self.K2_GetActorLocation` (stale `self.ReceiveActorBeginOverlap` _aspushing_box_3)) (- (+ (* (`self.GetActorForwardVector` _returnvalue) 150.0) (`self.K2_GetActorLocation` _returnvalue)) (0.0 0.0 50.0)) (`GameplayStatics.GetWorldDeltaSeconds`)))
    (if (`self.RKeyIsPressed`)
      (`KismetSystemLibrary.K2_ClearAndInvalidateTimerHandle` (stale `Key|E` _returnvalue_7))
      (set `self.IsPushingObject` false))))

(event `UpdateLocationPushingBox4`
  (bind _returnvalue (`GameplayStatics.GetPlayerCharacter` 0))
  ;[1 1 1] Box PickUp
  ;;[1 1 1] Side 4
  (if true
    (`self.K2_SetActorLocationAndRotation` :`self` (stale `self.ReceiveActorBeginOverlap` _aspushing_box_4) :`NewLocation` (`KismetMathLibrary.VInterpTo` (`self.K2_GetActorLocation` (stale `self.ReceiveActorBeginOverlap` _aspushing_box_4)) (- (+ (* (`self.GetActorForwardVector` _returnvalue) 150.0) (`self.K2_GetActorLocation` _returnvalue)) (0.0 0.0 50.0)) (`GameplayStatics.GetWorldDeltaSeconds`)))
    (if (`self.RKeyIsPressed`)
      (`KismetSystemLibrary.K2_ClearAndInvalidateTimerHandle` (stale `Key|E` _returnvalue_8))
      (set `self.IsPushingObject` false))))

(event `self.ReceiveActorEndOverlap`
  (params (OtherActor :type "Actor Object Reference"))
  ;[1 1 1] Box PickUp
  (cast `/Game/Blueprints/Pushing_Box` OtherActor)
  (`|ExecutionSequence`
    (:`then_0`
      (goto _label :!via `Close`))
    (:`then_1`
      (goto _label_2 :!via `Close`))
    (:`then_2`
      (goto _label_3 :!via `Close`))
    (:`then_3`
      (goto _label_4 :!via `Close`))))

(fn `UserConstructionScript`)