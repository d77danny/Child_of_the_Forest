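; BP_GravRemove is a trigger volume that switches off gravity for BP_Ghost while it is inside a box.
; On overlap begin, it constrains the ghost's CharacterMovement to a Z-axis plane and zeroes gravity scale; on overlap end, it releases the constraint and restores normal gravity.
; The gravity helpers act on the first BP_Ghost found via GetAllActorsOfClass rather than the overlapping actor.
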(event `self.Box.OnComponentBeginOverlap`
  (params (OverlappedComponent :type "PrimitiveComponent Object Reference") (OtherActor :type "Actor Object Reference") (OtherComp :type "PrimitiveComponent Object Reference") (OtherBodyIndex :type Integer) (bFromSweep :type Boolean) (SweepResult :type "HitResult Structure (by ref)"))
  (bind _asbp_ghost (cast `/Game/Blueprints/BP_Ghost` OtherActor))
  (bind _charactermovement (`Character.CharacterMovement` _asbp_ghost))
  (`MovementComponent.SetPlaneConstraintAxisSetting` _charactermovement "Z")
  (`MovementComponent.SetPlaneConstraintEnabled` _charactermovement true)
  (`self.Remove Gravity`))

(event `self.Box.OnComponentEndOverlap`
  (params (OverlappedComponent :type "PrimitiveComponent Object Reference") (OtherActor :type "Actor Object Reference") (OtherComp :type "PrimitiveComponent Object Reference") (OtherBodyIndex :type Integer))
  (bind _asbp_ghost (cast `/Game/Blueprints/BP_Ghost` OtherActor))
  (`MovementComponent.SetPlaneConstraintEnabled` (`Character.CharacterMovement` _asbp_ghost) false)
  (`self.Add Gravity`))

(fn `Add Gravity`
  (bind _outactors (`GameplayStatics.GetAllActorsOfClass` "/Game/Blueprints/BP_Ghost.BP_Ghost_C"))
  (set `CharacterMovementComponent.GravityScale` 1.0 (`Character.CharacterMovement` (`|GetArrayItem` _outactors))))

(fn `Remove Gravity`
  (bind _outactors (`GameplayStatics.GetAllActorsOfClass` "/Game/Blueprints/BP_Ghost.BP_Ghost_C"))
  (set `CharacterMovementComponent.GravityScale` 0.0 (`Character.CharacterMovement` (`|GetArrayItem` _outactors))))

(fn `UserConstructionScript`)