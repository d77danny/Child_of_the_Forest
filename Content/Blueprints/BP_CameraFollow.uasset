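; BP_CameraFollow is a camera-follow actor that moves itself to a target actor's location plus per-axis offsets.
; Tick follows Target2, while two identical custom events apply the same logic to Target1 but are not called within this graph.
; BeginPlay clears Target1, and the Switch input alternates through a FlipFlop between clearing Target1 and Target2.
; No assignment of a valid target or validity check appears in the graphs.
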(event `CustomEvent_1`
  (params (DeltaSeconds :type "Float (double-precision)"))
  (`self.K2_SetActorLocation` (`KismetMathLibrary.MakeVector` (+ (.x (`self.K2_GetActorLocation` (stale `self.ReceiveBeginPlay` _output_get))) (`self.Offset X`)) (+ (.y (`self.K2_GetActorLocation` (stale `self.ReceiveBeginPlay` _output_get))) (`self.Offset Y`)) (+ (.z (`self.K2_GetActorLocation` (stale `self.ReceiveBeginPlay` _output_get))) (`self.Offset Z`)))))

(event `self.ReceiveBeginPlay`
  (bind _output_get (set `self.Target1` null)))

(event `CustomEvent`
  (params (DeltaSeconds :type "Float (double-precision)"))
  (`self.K2_SetActorLocation` (`KismetMathLibrary.MakeVector` (+ (.x (`self.K2_GetActorLocation` (stale `InputAction|Switch` _output_get))) (`self.Offset X`)) (+ (.y (`self.K2_GetActorLocation` (stale `InputAction|Switch` _output_get))) (`self.Offset Y`)) (+ (.z (`self.K2_GetActorLocation` (stale `InputAction|Switch` _output_get))) (`self.Offset Z`)))))

(event `InputAction|Switch`
  (params (Key :type "Key Structure"))
  (:`Pressed`
    (`/Engine/EditorBlueprintResources/StandardMacros.FlipFlop`
      (:`A`
        (bind _output_get (set `self.Target1` null)))
      (:`B`
        (bind _output_get_2 (set `self.Target2` null))))))

(event `self.ReceiveTick`
  (params (DeltaSeconds :type "Float (single-precision)"))
  (`self.K2_SetActorLocation` (`KismetMathLibrary.MakeVector` (+ (.x (`self.K2_GetActorLocation` (stale `InputAction|Switch` _output_get_2))) (`self.Offset X`)) (+ (.y (`self.K2_GetActorLocation` (stale `InputAction|Switch` _output_get_2))) (`self.Offset Y`)) (+ (.z (`self.K2_GetActorLocation` (stale `InputAction|Switch` _output_get_2))) (`self.Offset Z`)))))

(fn `UserConstructionScript`)