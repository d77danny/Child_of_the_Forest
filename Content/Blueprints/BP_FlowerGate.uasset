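; BP_FlowerGate is an early flower gate actor with placeholder interaction for the player's ghost pawn.
; On BeginPlay it binds its empty Interact event to BP_Ghost's Interact dispatcher.
; Overlap with the Flower1 component toggles an interactable flag.
; A separate Interact input action reads that flag and only prints debug text, with no gate-opening logic yet.
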(event `Subscribe`
  (bind _asbp_ghost (cast `/Game/Blueprints/BP_Ghost` (`GameplayStatics.GetPlayerPawn` 0)))
  (add `/Game/Blueprints/BP_Ghost.Interact` _asbp_ghost (delegate `Interact`)))

(event `self.ReceiveBeginPlay`
  (`self.Subscribe`))

(event `Interact`)

(event `InputAction|Interact`
  (params (Key :type "Key Structure"))
  (:`Pressed`
    (if (`self.F1IsInteractable`)
      (`KismetSystemLibrary.PrintString` "F1 open")
      (else
        (`KismetSystemLibrary.PrintString` "Hello")))))

(event `self.Flower 1.OnComponentBeginOverlap`
  (params (OverlappedComponent :type "PrimitiveComponent Object Reference") (OtherActor :type "Actor Object Reference") (OtherComp :type "PrimitiveComponent Object Reference") (OtherBodyIndex :type Integer) (bFromSweep :type Boolean) (SweepResult :type "HitResult Structure (by ref)"))
  (set `self.F1IsInteractable` true))

(event `self.Flower 1.OnComponentEndOverlap`
  (params (OverlappedComponent :type "PrimitiveComponent Object Reference") (OtherActor :type "Actor Object Reference") (OtherComp :type "PrimitiveComponent Object Reference") (OtherBodyIndex :type Integer))
  (set `self.F1IsInteractable` false))

(fn `UserConstructionScript`)