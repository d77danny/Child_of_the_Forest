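; BP_TreeButtonGhost is an interactable that knocks down its BigTree, in a folder of buttons that work with the ghost.
; Overlap by a BP_Ghost prints a left-click prompt; Interact checks only IsInteractable, which this graph never clears.
; Interact prints a crack message, snaps the tree's relative location to its world location plus an offset, then rolls it over with the TreeFall timeline.
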(event `self.ReceiveActorBeginOverlap`
  (params (OtherActor :type "Actor Object Reference"))
  (cast `/Game/Blueprints/BP_Ghost` OtherActor)
  (`KismetSystemLibrary.PrintString` "Left mouse press to knock down tree"))

(event `self.Interact`
  (if (`self.bIsInteractable`)
    (`KismetSystemLibrary.PrintString` "*Crack*")
    (`self.K2_SetActorRelativeLocation` (`self.Big Tree`) (+ (`self.K2_GetActorLocation` (`self.Big Tree`)) (0.0 50.0 -130.0)) false false)
    (bind (_direction _alpha) (`Timeline|Tree Fall`)
      (:`Update`
        (`self.K2_SetActorRelativeRotation` (`self.Big Tree`) (`KismetMathLibrary.MakeRotator` _alpha) false false)))))

(fn `UserConstructionScript`
  (`parent.UserConstructionScript`))