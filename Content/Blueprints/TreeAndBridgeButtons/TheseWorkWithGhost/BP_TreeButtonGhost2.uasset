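; BP_TreeButtonGhost2 is an interactable trigger that knocks down a tree, with a prompt for the ghost character.
; Overlap by BP_Ghost prints a left-click hint, while Interact checks IsInteractable and runs a DoOnce.
; The fall plays a sound at world origin, lowers BigTree2 and pitches it over with the TreeFall2 timeline.
; The drop feeds the tree's world location, offset downward, into its relative location.
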(event `self.ReceiveActorBeginOverlap`
  (params (OtherActor :type "Actor Object Reference"))
  (cast `/Game/Blueprints/BP_Ghost` OtherActor)
  (`KismetSystemLibrary.PrintString` "Left mouse press to knock down tree"))

(event `self.Interact`
  (if (`self.bIsInteractable`)
    (`/Engine/EditorBlueprintResources/StandardMacros.DoOnce` false
      (:`Completed`
        (`|ExecutionSequence`
          (:`then_0`
            (`GameplayStatics.PlaySoundAtLocation` "/Game/Audio/SFX/object_tree_fall.object_tree_fall" (0.0 0.0 0.0) (struct) 1.0 1.0 0.0 null null null))
          (:`then_1`
            (`KismetSystemLibrary.PrintString` "*Crack*")
            (`self.K2_SetActorRelativeLocation` (`self.Big Tree 2`) (+ (`self.K2_GetActorLocation` (`self.Big Tree 2`)) (0.0 0.0 -55.0)) false false)
            (bind (_direction _alpha) (`Timeline|Tree Fall 2`)
              (:`Update`
                (`self.K2_SetActorRelativeRotation` (`self.Big Tree 2`) (`KismetMathLibrary.MakeRotator` 0.0 _alpha) false false)))))))))

(fn `UserConstructionScript`
  (`parent.UserConstructionScript`))