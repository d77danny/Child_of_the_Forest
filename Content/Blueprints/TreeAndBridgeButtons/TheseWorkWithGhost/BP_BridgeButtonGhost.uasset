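; BP_BridgeButtonGhost is a button that raises a linked bridge, prompting the player to left-click when BP_Ghost overlaps it.
; Interact, gated by IsInteractable and a DoOnce, adds button audio, fires FocusOnWitch and BridgeIsMoving, then plays the Raise timeline.
; The timeline drives MovingBridge's relative Z, feeding its world X/Y back as relative values.
; On finish, it plays a drag sound at world origin and fires BridgeIsMoving again.
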(event `self.ReceiveActorBeginOverlap`
  (params (OtherActor :type "Actor Object Reference"))
  (cast `/Game/Blueprints/BP_Ghost` OtherActor)
  (`KismetSystemLibrary.PrintString` "Left mouse click to raise the bridge"))

(event `self.Interact`
  (bind _moving_bridge (`self.Moving Bridge`))
  (bind (_returnvalue_x _returnvalue_y) (`KismetMathLibrary.BreakVector` (`self.K2_GetActorLocation` _moving_bridge)))
  (if (`self.bIsInteractable`)
    (`/Engine/EditorBlueprintResources/StandardMacros.DoOnce` false
      (:`Completed`
        (`AddComponent|NODE_AddAudioComponent-0`) ; This plays a sound when pressing the bridge button.
        (`self.FocusOnWitch`)
        (`self.BridgeIsMoving`)
        (bind (_direction _alpha) (`Timeline|Raise`)
          (:`Update`
            (`self.K2_SetActorRelativeLocation` _moving_bridge (`KismetMathLibrary.MakeVector` _returnvalue_x _returnvalue_y _alpha) false false))
          (:`Finished`
            (`GameplayStatics.PlaySoundAtLocation` "/Game/Audio/SFX/object_drag.object_drag" (0.0 0.0 0.0) (struct) 1.0 1.0 0.0 null null null) ; This supposed to play as the bridge rises.\nI can only seems to put sounds in the middle of node links.\nPutting this into Raise's Update will cause the audio to glitch.
            (`self.BridgeIsMoving`)))))))

(fn `UserConstructionScript`
  (`parent.UserConstructionScript`))