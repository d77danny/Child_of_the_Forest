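; Pushable box actor that tells the BP_Witch character which way to push it.
; Four side overlap volumes each flag their side on entry and write a fixed axis-aligned direction to the witch's SetPushDirection variable.
; Leaving a volume clears only that side's flag, so the witch keeps the last direction.
; The box's graph contains no movement logic.
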(event `self.ReceiveBeginPlay`)

(event `self.Side1.OnComponentBeginOverlap`
  (params (OverlappedComponent :type "PrimitiveComponent Object Reference") (OtherActor :type "Actor Object Reference") (OtherComp :type "PrimitiveComponent Object Reference") (OtherBodyIndex :type Integer) (bFromSweep :type Boolean) (SweepResult :type "HitResult Structure (by ref)"))
  ;[1 1 1] Box PickUp Overlaps
  (bind _asbp_witch (cast `/Game/Blueprints/BP_Witch` OtherActor))
  (set `self.Side_1` true)
  (set `/Game/Blueprints/BP_Witch.SetPushDirection` (-1.0 0.0 0.0) _asbp_witch))

(event `self.ReceiveActorBeginOverlap`
  (params (OtherActor :type "Actor Object Reference")))

(event `self.Side1.OnComponentEndOverlap`
  (params (OverlappedComponent :type "PrimitiveComponent Object Reference") (OtherActor :type "Actor Object Reference") (OtherComp :type "PrimitiveComponent Object Reference") (OtherBodyIndex :type Integer))
  ;[1 1 1] Box PickUp Overlaps
  (cast `/Game/Blueprints/BP_Witch` OtherActor)
  (set `self.Side_1` false))

(event `self.ReceiveTick`
  (params (DeltaSeconds :type "Float (single-precision)")))

(event `self.Side2.OnComponentBeginOverlap`
  (params (OverlappedComponent :type "PrimitiveComponent Object Reference") (OtherActor :type "Actor Object Reference") (OtherComp :type "PrimitiveComponent Object Reference") (OtherBodyIndex :type Integer) (bFromSweep :type Boolean) (SweepResult :type "HitResult Structure (by ref)"))
  ;[1 1 1] Box PickUp Overlaps
  (bind _asbp_witch (cast `/Game/Blueprints/BP_Witch` OtherActor))
  (set `self.Side_2` true)
  (set `/Game/Blueprints/BP_Witch.SetPushDirection` (-0.0 1.0 0.0) _asbp_witch))

(event `self.Side2.OnComponentEndOverlap`
  (params (OverlappedComponent :type "PrimitiveComponent Object Reference") (OtherActor :type "Actor Object Reference") (OtherComp :type "PrimitiveComponent Object Reference") (OtherBodyIndex :type Integer))
  ;[1 1 1] Box PickUp Overlaps
  (cast `/Game/Blueprints/BP_Witch` OtherActor)
  (set `self.Side_2` false))

(event `self.Side 3.OnComponentBeginOverlap`
  (params (OverlappedComponent :type "PrimitiveComponent Object Reference") (OtherActor :type "Actor Object Reference") (OtherComp :type "PrimitiveComponent Object Reference") (OtherBodyIndex :type Integer) (bFromSweep :type Boolean) (SweepResult :type "HitResult Structure (by ref)"))
  ;[1 1 1] Box PickUp Overlaps
  (bind _asbp_witch (cast `/Game/Blueprints/BP_Witch` OtherActor))
  (set `self.Side_3` true)
  (set `/Game/Blueprints/BP_Witch.SetPushDirection` (1.0 0.0 0.0) _asbp_witch))

(event `self.Side 3.OnComponentEndOverlap`
  (params (OverlappedComponent :type "PrimitiveComponent Object Reference") (OtherActor :type "Actor Object Reference") (OtherComp :type "PrimitiveComponent Object Reference") (OtherBodyIndex :type Integer))
  ;[1 1 1] Box PickUp Overlaps
  (cast `/Game/Blueprints/BP_Witch` OtherActor)
  (set `self.Side_3` false))

(event `self.Side 4.OnComponentBeginOverlap`
  (params (OverlappedComponent :type "PrimitiveComponent Object Reference") (OtherActor :type "Actor Object Reference") (OtherComp :type "PrimitiveComponent Object Reference") (OtherBodyIndex :type Integer) (bFromSweep :type Boolean) (SweepResult :type "HitResult Structure (by ref)"))
  ;[1 1 1] Box PickUp Overlaps
  (bind _asbp_witch (cast `/Game/Blueprints/BP_Witch` OtherActor))
  (set `self.Side_4` true)
  (set `/Game/Blueprints/BP_Witch.SetPushDirection` (0.0 -1.0 0.0) _asbp_witch))

(event `self.Side 4.OnComponentEndOverlap`
  (params (OverlappedComponent :type "PrimitiveComponent Object Reference") (OtherActor :type "Actor Object Reference") (OtherComp :type "PrimitiveComponent Object Reference") (OtherBodyIndex :type Integer))
  ;[1 1 1] Box PickUp Overlaps
  (cast `/Game/Blueprints/BP_Witch` OtherActor)
  (set `self.Side_4` false))

(fn `UserConstructionScript`)